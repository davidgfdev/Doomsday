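; BP_Nihilist_Ammo is an ammo pickup actor, shown as a sprite, that gives ammo to BP_Sen.
; Each tick it turns the whole actor on yaw only to face player pawn 0, billboarding the sprite upright.
; Overlapping its Box calls AddAmmo with a fixed amount on BP_Sen; the graph never destroys or disables the pickup, so each new overlap grants ammo again.
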(event OnComponentBeginOverlap(Box)
  (params (OverlappedComponent :type Primitive%20Component%20Object%20Reference) (OtherActor :type Actor%20Object%20Reference) (OtherComp :type Primitive%20Component%20Object%20Reference) (OtherBodyIndex :type Integer) (bFromSweep :type Boolean) (SweepResult :type Hit%20Result%20Structure%20%28by%20ref%29))
  (bind _asbp_sen (Utilities|Casting|CastToBP_Sen OtherActor))
  (Class|Sen|AddAmmo _asbp_sen 5e+01))

(event EventTick
  (params (DeltaSeconds :type Float%20%28single-precision%29))
  (bind _returnvalue (Game|Player|GetPlayerPawn 0))
  (Utilities|IsValid _returnvalue
    (:Is%20Valid
      (Transformation|SetActorRotation (Math|Rotator|MakeRotator 0.0 0.0 (.Yaw (Math|Rotator|BreakRotator (Math|Rotator|FindLookatRotation (Transformation|GetWorldLocation (Variables|Default|GetNihilist_Sprite)) (Transformation|GetActorLocation _returnvalue)))))))))

(fn ConstructionScript)