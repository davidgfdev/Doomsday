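; BP_Inscription is a level trigger that acts as both a checkpoint and a lore inscription for the BP_Sen character.
; On Box overlap, it sends its RespawnPoint location to the ASCENDENTE game mode as the new respawn location, then shows a WBP_Inscription widget filled with its Lore.
; When BP_Sen leaves the box, it removes every top-level WBP_Inscription widget from the screen.
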(event OnComponentBeginOverlap(Box)
  (params (OverlappedComponent :type Primitive%20Component%20Object%20Reference) (OtherActor :type Actor%20Object%20Reference) (OtherComp :type Primitive%20Component%20Object%20Reference) (OtherBodyIndex :type Integer) (bFromSweep :type Boolean) (SweepResult :type Hit%20Result%20Structure%20%28by%20ref%29))
  (Utilities|Casting|CastToBP_Sen OtherActor)
  (bind _asascendentegame_mode_base (Utilities|Casting|CastToASCENDENTEGameModeBase (Game|GetGameMode)))
  (Class|ASCENDENTEGameModeBase|SetRespawnLocation _asascendentegame_mode_base (Transformation|GetWorldLocation (Variables|Default|GetRespawnPoint)))
  (bind _returnvalue (UserInterface|CreateWidget "/Game/Blueprints/Widgets/WBP_Inscription.WBP_Inscription_C"))
  (Default|SetLore _returnvalue (Variables|Default|GetLore))
  (UserInterface|Viewport|AddtoPlayerScreen _returnvalue))

(event OnComponentEndOverlap(Box)
  (params (OverlappedComponent :type Primitive%20Component%20Object%20Reference) (OtherActor :type Actor%20Object%20Reference) (OtherComp :type Primitive%20Component%20Object%20Reference) (OtherBodyIndex :type Integer))
  (Utilities|Casting|CastToBP_Sen OtherActor)
  (bind _foundwidgets (Widget|GetAllWidgetsOfClass "/Game/Blueprints/Widgets/WBP_Inscription.WBP_Inscription_C" true))
  (for _array_element _foundwidgets
    (Widget|RemovefromParent _array_element)))

(fn ConstructionScript)