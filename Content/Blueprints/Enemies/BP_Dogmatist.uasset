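; BP_Dogmatist is a 2D flipbook enemy that supplies the animation, AI state and health display responses for its character.
; Death and attack events play non-looping Faithful flipbooks, and a finished attack returns to the looping idle.
; Update events copy line-of-fire, aggro and death flags into the AI controller's Blackboard.
; Health updates feed the enemy health widget with a hardcoded maximum, and debug prints remain in death and line-of-fire events.
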(event OnFinishedPlaying(EnemySpriteFlipbook)
  (bind _enemyspriteflipbook (Variables|Default|GetEnemySpriteFlipbook))
  (if (== (Class|PaperFlipbookComponent|GetFlipbook _enemyspriteflipbook) "/Game/Sprites/Faithful/Attack/PF_Faithful_Attack.PF_Faithful_Attack")
    (Sprite|SetFlipbook _enemyspriteflipbook "/Game/Sprites/Faithful/Idle/PF_Faithful_Idle.PF_Faithful_Idle")
    (Components|Timeline|SetLooping _enemyspriteflipbook true)))

(event EventPlayDeathAnimation
  (bind _enemyspriteflipbook (Variables|Default|GetEnemySpriteFlipbook))
  (Development|PrintString "Muelto")
  (Sprite|SetFlipbook _enemyspriteflipbook "/Game/Sprites/Faithful/Death/PF_Faithful_Death.PF_Faithful_Death")
  (Components|Timeline|SetLooping _enemyspriteflipbook false))

(event EventPlayAttackAnimation
  (bind _enemyspriteflipbook (Variables|Default|GetEnemySpriteFlipbook))
  (Sprite|SetFlipbook _enemyspriteflipbook "/Game/Sprites/Faithful/Attack/PF_Faithful_Attack.PF_Faithful_Attack")
  (Components|Timeline|SetLooping _enemyspriteflipbook false))

(event EventUpdateBlackboardAggro
  (AI|Components|Blackboard|SetValueasBool (AI|GetBlackboard (AI|GetAIController self)) (Utilities|Name|MakeLiteralName "isPlayerAggro") (Variables|Default|GetdoesPlayerHasAggro)))

(event EventUpdateHealth
  (params (Health :type Float%20%28single-precision%29))
  (bind _aswbp_enemy_health (Utilities|Casting|CastToWBP_EnemyHealth (UserInterface|GetWidget (Variables|Default|GetHealthWidget))))
  (Default|SetHealth _aswbp_enemy_health Health 1e+02))

(event EventUpdateBlackboardLineOfFire
  (bind _isplayerinlineoffire (Variables|Default|GetisPlayerInLineOfFire))
  (AI|Components|Blackboard|SetValueasBool (AI|GetBlackboard (AI|GetAIController self)) (Utilities|Name|MakeLiteralName "isPlayerInLineOfFire") _isplayerinlineoffire)
  (Development|PrintString (Utilities|String|ToString(Boolean) _isplayerinlineoffire)))

(event EventUpdateIsDead
  (AI|Components|Blackboard|SetValueasBool (AI|GetBlackboard (AI|GetAIController self)) (Utilities|Name|MakeLiteralName "isDead") (Variables|Default|GetisDead)))

(fn ConstructionScript)