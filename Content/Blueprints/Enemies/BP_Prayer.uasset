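; BP_Prayer is the Blueprint for the Prayer enemy, handling its Paper2D flipbook animations and AI state updates.
; Death and attack events swap the flipbook and play it non-looping from the first frame.
; When the attack flipbook finishes, the sprite returns to looping idle.
; Separate update events copy player aggro and death flags into the AI controller's Blackboard.
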(event OnFinishedPlaying(EnemySpriteFlipbook)
  (bind _enemyspriteflipbook (Variables|Default|GetEnemySpriteFlipbook))
  (if (== (Class|PaperFlipbookComponent|GetFlipbook _enemyspriteflipbook) "/Game/Sprites/Prayer/Attack/PF_Prayer_Attack.PF_Prayer_Attack")
    (Sprite|SetFlipbook _enemyspriteflipbook "/Game/Sprites/Prayer/Idle/PF_Prayer_Idle.PF_Prayer_Idle")
    (Components|Timeline|SetLooping _enemyspriteflipbook true)
    (Audio|Components|Audio|Play _enemyspriteflipbook)))

(event EventPlayDeathAnimation
  (bind _enemyspriteflipbook (Variables|Default|GetEnemySpriteFlipbook))
  (Sprite|SetFlipbook _enemyspriteflipbook "/Game/Sprites/Prayer/Death/PF_Prayer_Death.PF_Prayer_Death")
  (Class|PaperFlipbookComponent|SetPlaybackPositioninFrames _enemyspriteflipbook 0 false)
  (Components|Timeline|SetLooping _enemyspriteflipbook false))

(event EventPlayAttackAnimation
  (bind _enemyspriteflipbook (Variables|Default|GetEnemySpriteFlipbook))
  (Sprite|SetFlipbook _enemyspriteflipbook "/Game/Sprites/Prayer/Attack/PF_Prayer_Attack.PF_Prayer_Attack")
  (Class|PaperFlipbookComponent|SetPlaybackPositioninFrames _enemyspriteflipbook 0 false)
  (Components|Timeline|SetLooping _enemyspriteflipbook false))

(event EventUpdateBlackboardAggro
  (AI|Components|Blackboard|SetValueasBool (AI|GetBlackboard (AI|GetAIController self)) (Utilities|Name|MakeLiteralName "isPlayerAggro") (Variables|Default|GetdoesPlayerHasAggro)))

(event EventUpdateIsDead
  (AI|Components|Blackboard|SetValueasBool (AI|GetBlackboard (AI|GetAIController self)) (Utilities|Name|MakeLiteralName "isDead") (Variables|Default|GetisDead)))

(fn ConstructionScript)