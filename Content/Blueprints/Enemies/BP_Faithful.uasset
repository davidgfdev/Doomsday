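; BP_Faithful is the Faithful enemy, an AI-controlled character animated with Paper2D flipbooks.
; Animation events play non-looping attack and death flipbooks from the first frame; death also stops movement, and a finished attack returns to looping idle.
; Update events copy player-in-range, aggro and death flags to the AI controller's blackboard.
; The construction script draws a debug sphere for aggro range; UpdateHealth is empty, with health-widget code left unconnected.
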(event OnFinishedPlaying(EnemySpriteFlipbook)
  (bind _enemyspriteflipbook (Variables|Default|GetEnemySpriteFlipbook))
  (if (== (Class|PaperFlipbookComponent|GetFlipbook _enemyspriteflipbook) "/Game/Sprites/Faithful/Attack/PF_Faithful_Attack.PF_Faithful_Attack")
    (Sprite|SetFlipbook _enemyspriteflipbook "/Game/Sprites/Faithful/Idle/PF_Faithful_Idle.PF_Faithful_Idle")
    (Components|Timeline|SetLooping _enemyspriteflipbook true)
    (Audio|Components|Audio|Play _enemyspriteflipbook)))

(event EventUpdateBlackboardPlayerinRange
  (AI|Components|Blackboard|SetValueasBool (AI|GetBlackboard (AI|GetAIController self)) (Utilities|Name|MakeLiteralName "IsPlayerInRange") (Variables|Default|GetisPlayerInRange)))

(event EventPlayDeathAnimation
  (bind _enemyspriteflipbook (Variables|Default|GetEnemySpriteFlipbook))
  (Development|PrintString "Muelto")
  (Sprite|SetFlipbook _enemyspriteflipbook "/Game/Sprites/Faithful/Death/PF_Faithful_Death.PF_Faithful_Death")
  (Components|Timeline|SetLooping _enemyspriteflipbook false)
  (Class|NavMovementComponent|StopActiveMovement (Variables|Character|GetCharacterMovement))
  (Class|PaperFlipbookComponent|SetPlaybackPositioninFrames _enemyspriteflipbook 0 false))

(event EventPlayAttackAnimation
  (bind _enemyspriteflipbook (Variables|Default|GetEnemySpriteFlipbook))
  (Sprite|SetFlipbook _enemyspriteflipbook "/Game/Sprites/Faithful/Attack/PF_Faithful_Attack.PF_Faithful_Attack")
  (Components|Timeline|SetLooping _enemyspriteflipbook false)
  (Class|PaperFlipbookComponent|SetPlaybackPositioninFrames _enemyspriteflipbook 0 false))

(event EventUpdateBlackboardAggro
  (AI|Components|Blackboard|SetValueasBool (AI|GetBlackboard (AI|GetAIController self)) (Utilities|Name|MakeLiteralName "isPlayerAggro") (Variables|Default|GetdoesPlayerHasAggro)))

(event EventUpdateHealth
  (params (Health :type Float%20%28single-precision%29)))

(event EventUpdateIsDead
  (AI|Components|Blackboard|SetValueasBool (AI|GetBlackboard (AI|GetAIController self)) (Utilities|Name|MakeLiteralName "isDead") (Variables|Default|GetisDead)))

(fn ConstructionScript
  (Rendering|Debug|DrawDebugSphere (Transformation|GetActorLocation) (Variables|Default|GetAggroRange) 12 "(R=1.000000,G=0.055031,B=0.000000,A=1.000000)" -1.0))