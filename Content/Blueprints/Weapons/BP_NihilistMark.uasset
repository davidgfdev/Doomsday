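; BP_NihilistMark is a weapon mark actor that detonates when damaged by a HopeAndPrison damage causer.
; That hit applies radial damage around the mark while ignoring itself, prints a debug message, then calls Explode.
; Explode only destroys the actor, so the timer set on BeginPlay removes an untriggered mark after a few seconds without dealing damage.
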(event Custom|Explode
  (Actor|DestroyActor))

(event Game|Damage|EventAnyDamage
  (params (Damage :type Float%20%28single-precision%29) (DamageType :type Damage%20Type%20Object%20Reference) (InstigatedBy :type Controller%20Object%20Reference) (DamageCauser :type Actor%20Object%20Reference))
  (Utilities|Casting|CastToHopeAndPrison DamageCauser)
  (Game|Damage|ApplyRadialDamage 4e+01 (Transformation|GetActorLocation) 1e+02 "/Script/Engine.DamageType" (Utilities|Array|MakeArray self) 0 0 false "ECC_Visibility")
  (Development|PrintString "Explosión")
  (CallFunction|Explode))

(event EventBeginPlay
  (Utilities|Time|SetTimerbyFunctionName 0 "Explode" 5.0))

(fn ConstructionScript)