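; BP_Sen is the player character Blueprint that links Sen's gameplay events to the WBP_Hud widget.
; Ammo, health and ascend-panel events push values to every HUD widget found, while damage and death events trigger HUD animations, with a camera shake on damage.
; BeginPlay caches the HUD and registers the spawn location as the game mode's respawn point.
; Each tick, a camera line trace switches the crosshair state when aimed at an Enemy.
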(event EventTick
  (params (DeltaSeconds :type Float%20%28single-precision%29))
  (bind _cameracomponent (Variables|Default|GetCameraComponent))
  (bind _hud (Variables|Default|GetHUD))
  (bind _returnvalue (Transformation|GetWorldLocation _cameracomponent))
  (bind _outhit (Collision|LineTraceByChannel _returnvalue (+ (* (Math|Vector|GetForwardVector _cameracomponent) 5000) _returnvalue) "TraceTypeQuery1" false 0 "None"))
  (Utilities|Casting|CastToEnemy (.HitActor (Collision|BreakHitResult _outhit))
    (:then
      (Default|SetCrosshairState _hud "NewEnumerator1"))
    (:CastFailed
      (Default|SetCrosshairState _hud "NewEnumerator0"))))

(event EventBeginPlay
  (bind _foundwidgets (Widget|GetAllWidgetsOfClass "/Game/Blueprints/Widgets/WBP_Hud.WBP_Hud_C" true))
  (for _array_element _foundwidgets
    (Variables|Default|SetHUD _array_element)
    (bind _asbp_ascendentegame_mode_base (Utilities|Casting|CastToBP_ASCENDENTEGameModeBase (Game|GetGameMode)))
    (Class|ASCENDENTEGameModeBase|SetRespawnLocation _asbp_ascendentegame_mode_base (Transformation|GetActorLocation))))

(event EventMakeDamageEffect
  (Default|TriggerDamageAnimation (Variables|Default|GetHUD))
  (Game|Feedback|ClientStartCameraShake (Game|GetPlayerController 0) "/Game/Blueprints/Camera/BP_Damage_HeadBob.BP_Damage_HeadBob_C" 5.0 "CameraLocal" "0, 0, 0"))

(event EventMakeDeathEffect
  (Default|TriggerDeathAnimation (Variables|Default|GetHUD)))

(event EventUpdateAmmo
  (params (Ammo :type Float%20%28single-precision%29))
  (bind _foundwidgets (Widget|GetAllWidgetsOfClass "/Game/Blueprints/Widgets/WBP_Hud.WBP_Hud_C" true))
  (for _array_element _foundwidgets
    (Default|SetAmmoBar _array_element Ammo)))

(event EventUpdateHealth
  (params (Health :type Float%20%28single-precision%29))
  (bind _foundwidgets (Widget|GetAllWidgetsOfClass "/Game/Blueprints/Widgets/WBP_Hud.WBP_Hud_C" true))
  (for _array_element _foundwidgets
    (Default|SetHealthBar _array_element Health 1e+02)))

(event EventUpdateAscendPanel
  (params (isVisible :type Boolean))
  (bind _foundwidgets (Widget|GetAllWidgetsOfClass "/Game/Blueprints/Widgets/WBP_Hud.WBP_Hud_C" true))
  (for _array_element _foundwidgets
    (Default|ShowAscendPanel _array_element isVisible)))

(fn ConstructionScript)